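; BP_Player is a player pawn with floating movement and a zoomable spring-arm camera.
; Each Tick, while Move is set and its X position has not dropped below TargetLoc, it drives itself along negative X; otherwise it stops immediately.
; ZoomCamera shortens or lengthens the spring arm by a speed-scaled amount, clamped between minimum and maximum lengths.
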(event `self.ReceiveTick`
  (params (DeltaSeconds :type "Float (single-precision)"))
  (bind _returnvalue_x (`KismetMathLibrary.BreakVector` (`self.K2_GetActorLocation`)))
  (if (and (`self.Move`) (not (> (`self.TargetLoc`) _returnvalue_x)))
    (`self.AddMovementInput` (10.0 0.0 0.0) -1.0)
    (else
      (`MovementComponent.StopMovementImmediately` (`self.FloatingPawnMovement`)))))

(fn `UserConstructionScript`)

(fn `ZoomCamera`
  (params (Amount :type "Float (double-precision)"))
  (set `SpringArmComponent.TargetArmLength` (`KismetMathLibrary.FClamp` (- (`SpringArmComponent.TargetArmLength` (`self.SpringArm`)) (* Amount (`self.CameraZoomSpeed`))) (`self.MinSpringArmLength`) (`self.MaxSpringArmLength`)) (`self.SpringArm`)))