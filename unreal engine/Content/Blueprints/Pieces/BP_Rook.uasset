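; BP_Rook is a chess rook piece Blueprint that defines which tiles the rook can move to.
; GetAvailableMoves calls GetTilesFromSlide from the start tile in four directions, each up to eight tiles, and appends the results into one returned array.
; The event graph holds only disabled default nodes, and the construction script only calls its parent.
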(fn `GetAvailableMoves`
  (params (StartTile :type "/Game/Blueprints/Board/Tile Structure"))
  (returns (DestinationTiles :type "Array of /Game/Blueprints/Board/Tile Structure"))
  (locals (Output :type "Array of /Game/Blueprints/Board/Tile Structure"))
  (`|ExecutionSequence`
    (:`then_0`
      (`|ExecutionSequence`
        (:`then_0`
          (bind _crossedtiles (`self.GetTilesFromSlide` (`local.StartTile`) "NewEnumerator0" 8))
          (`KismetArrayLibrary.Array_Append` (`local.Output`) _crossedtiles))
        (:`then_1`
          (bind _crossedtiles_2 (`self.GetTilesFromSlide` (`local.StartTile`) "NewEnumerator3" 8))
          (`KismetArrayLibrary.Array_Append` (`local.Output`) _crossedtiles_2))
        (:`then_2`
          (bind _crossedtiles_3 (`self.GetTilesFromSlide` (`local.StartTile`) "NewEnumerator6" 8))
          (`KismetArrayLibrary.Array_Append` (`local.Output`) _crossedtiles_3))
        (:`then_3`
          (bind _crossedtiles_4 (`self.GetTilesFromSlide` (`local.StartTile`) "NewEnumerator2" 8))
          (`KismetArrayLibrary.Array_Append` (`local.Output`) _crossedtiles_4))))
    (:`then_1`
      (return (`local.Output`)))))

(fn `UserConstructionScript`
  (`parent.UserConstructionScript`))