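; Base piece for a two-player, chess-like board game, tinted by owner colour, with player 1's pieces rotated 180 degrees.
; GetAvailableMoves is an empty stub, alongside helpers for single-step moves and eight-direction slides up to a maximum distance.
; Both use GetTileAfterMove for owner-relative offsets and CanTileBeMovedTo to check board validity, occupancy and capture mode.
; The piece also stores its column, row and whether it has ever moved.
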(event `self.ReceiveBeginPlay`
  (bind _returnvalue (`KismetMaterialLibrary.CreateDynamicMaterialInstance` "/Game/Assets/M_Piece.M_Piece"))
  (`PrimitiveComponent.SetMaterial` (`self.StaticMesh`) 0 _returnvalue)
  (`MaterialInstanceDynamic.SetVectorParameterValue` _returnvalue "Color" (`/Game/Blueprints/ChessLibrary.GetPlayerColor` (`self.OwningPlayerIndex`)))
  (if (== (`self.OwningPlayerIndex`) 1)
    (`self.K2_SetActorRotation` (struct :`Yaw` 180.0))))

(event `OnMoved`
  (set `self.HasEverMoved` true))

(fn `CanTileBeMovedTo?`
  (params (Tile :type "/Game/Blueprints/Board/Tile Structure") (CaptureMode :type "/Game/Blueprints/ECaptureMode Enum" :default "NewEnumerator0"))
  (returns (Result :type Boolean) (LastInLine :type Boolean))
  (locals (`LastInLine (local)` :type Boolean) (`Add (local)` :type Boolean))
  (`|ExecutionSequence`
    (:`then_0`
      (bind (_tilevalid _tilefree _piece) (`/Game/Blueprints/Board/BP_Board.GetTileData` (`/Game/Blueprints/ChessLibrary.GetBoard` (`self.board`)) (`local.Tile`)))
      (if _tilevalid
        (if _tilefree
          (if (`|EnumEquality` (`local.CaptureMode`) "NewEnumerator2")
            (set `local.LastInLine (local)` true)
            (else
              (set `local.Add (local)` true :!label _label)))
          (else
            (set `local.LastInLine (local)` true)
            (if (and (`|EnumInequality` (`local.CaptureMode`) "NewEnumerator1") (!= (`/Game/Blueprints/Pieces/BP_Piece.OwningPlayerIndex` _piece) (`self.OwningPlayerIndex`)))
              (goto _label))))
        (else
          (set `local.LastInLine (local)` true))))
    (:`then_1`
      (return (`local.Add (local)`) (`local.LastInLine (local)`)))))

(fn `GetAvailableMoves`
  (params (StartTile :type "/Game/Blueprints/Board/Tile Structure"))
  (returns (DestinationTiles :type "Array of /Game/Blueprints/Board/Tile Structure"))
  (return))

(fn `GetHasEverMoved`
  (returns (HasEverMoved :type Boolean))
  (return (`self.HasEverMoved`)))

(fn `GetTileAfterMove`
  (params (Tile :type "/Game/Blueprints/Board/Tile Structure") (Forward :type Integer :default 1) (Right :type Integer))
  (returns (NewTile :type "/Game/Blueprints/Board/Tile Structure"))
  (bind _returnvalue (select `int` (`self.OwningPlayerIndex`) :`0` 1 :`1` -1))
  (return (make `/Game/Blueprints/Board/Tile` (+ Tile_Col_2_767D76F24B6395F8CD2202A2E588D57E (* (`local.Right`) _returnvalue)) (+ Tile_Row_4_A31AD37F4ABEE7282C2022A30B0EBA3F (* _returnvalue (`local.Forward`))))))

(fn `GetTilesFromMove`
  (params (Tile :type "/Game/Blueprints/Board/Tile Structure") (Forward :type Integer) (Right :type Integer) (CaptureMode :type "/Game/Blueprints/ECaptureMode Enum" :default "NewEnumerator0"))
  (returns (Tiles :type "Array of /Game/Blueprints/Board/Tile Structure"))
  (locals (CurrentTile :type "/Game/Blueprints/Board/Tile Structure"))
  (bind _newtile (`self.GetTileAfterMove` Tile Forward Right))
  (bind _output_get (set `local.CurrentTile` _newtile))
  (bind _result (`self.CanTileBeMovedTo?` _output_get (`local.CaptureMode`)))
  (if _result
    (return (`|MakeArray` (`local.CurrentTile`)))
    (else
      (return))))

(fn `GetTilesFromSlide`
  (params (Tile :type "/Game/Blueprints/Board/Tile Structure") (Direction :type "/Game/Blueprints/ESlideDirection Enum" :default "NewEnumerator0") (MaxDistance :type Integer) (CaptureMode :type "/Game/Blueprints/ECaptureMode Enum" :default "NewEnumerator0"))
  (returns (CrossedTiles :type "Array of /Game/Blueprints/Board/Tile Structure"))
  (locals (CurrentTile :type "/Game/Blueprints/Board/Tile Structure") (Loop :type Boolean :default true) (Output :type "Array of /Game/Blueprints/Board/Tile Structure") (Distance :type Integer))
  (set `local.CurrentTile` Tile)
  (while (and (`local.Loop`) (< (`local.Distance`) (`local.MaxDistance`)))
    (`/Engine/EditorBlueprintResources/StandardMacros.IncrementInt` (`local.Distance`)
      (:`  `
        (bind _newtile (`self.GetTileAfterMove` (`local.CurrentTile`) (select `/Game/Blueprints/ESlideDirection` (`local.Direction`) :`NewEnumerator0` 1 :`NewEnumerator4` 1 :`NewEnumerator1` -1 :`NewEnumerator2` -1 :`NewEnumerator5` -1 :`NewEnumerator7` 1) (select `/Game/Blueprints/ESlideDirection` (`local.Direction`) :`NewEnumerator4` 1 :`NewEnumerator3` 1 :`NewEnumerator1` 1 :`NewEnumerator5` -1 :`NewEnumerator6` -1 :`NewEnumerator7` -1)))
        (bind _output_get (set `local.CurrentTile` _newtile))
        (bind (_result _lastinline) (`self.CanTileBeMovedTo?` _output_get (`local.CaptureMode`)))
        (set `local.Loop` (not _lastinline))
        (if _result
          (`KismetArrayLibrary.Array_Add` (`local.Output`) (`local.CurrentTile`))))))
  (return (`local.Output`)))

(fn `SetLoc`
  (params (Col :type Integer) (Row :type Integer))
  (set `self.Col` Col)
  (set `self.Row` Row))

(fn `UserConstructionScript`)