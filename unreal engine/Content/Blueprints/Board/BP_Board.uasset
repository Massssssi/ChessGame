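; Chess board actor that, on the authority only, spawns both players' pieces at BeginPlay and tracks them in a flat 64-slot BoardState array.
; Helpers convert between tiles and world positions on a grid centered on the actor.
; Move checks defer to each piece's GetAvailableMoves; PerformMove teleports the piece, destroys any captured one and updates the array.
; GetRandomMove retries random array picks until it finds a legal move for player index 1.
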(event `self.ReceiveBeginPlay`
  (`/Engine/EditorBlueprintResources/ActorMacros.Switch Has Authority`
    (:`Authority`
      (`KismetArrayLibrary.Array_Resize` (`self.BoardState`) 64)
      (for _index (range 2)
        (`self.Spawn Pawns` _index)
        (`self.SpawnRooks` _index)
        (`self.SpawnKnights` _index)
        (`self.SpawnBishops` _index)
        (`self.SpawnQueens` _index)
        (`self.SpawnKings` _index)))))

(fn `BoardStateAddPiece`
  (params (Item :type "/Game/Blueprints/Pieces/BP_Piece Object Reference (by ref)") (Tile :type "/Game/Blueprints/Board/Tile Structure"))
  (`KismetArrayLibrary.Array_Set` (`self.BoardState`) (`self.TileToIndex` Tile) Item))

(fn `BoardStateMovePiece`
  (params (StartTile :type "/Game/Blueprints/Board/Tile Structure") (DestinationTile :type "/Game/Blueprints/Board/Tile Structure"))
  (locals (PieceToMove :type "/Game/Blueprints/Pieces/BP_Piece Object Reference"))
  (set `local.PieceToMove` (`self.GetPieceAtTile` StartTile))
  (`KismetArrayLibrary.Array_Set` (`self.BoardState`) (`self.TileToIndex` (`local.StartTile`)))
  (`KismetArrayLibrary.Array_Set` (`self.BoardState`) (`self.TileToIndex` (`local.DestinationTile`)) (`local.PieceToMove`))
  (`/Game/Blueprints/Pieces/BP_Piece.OnMoved` (`local.PieceToMove`)))

(fn `CanPerformMove?`
  (params (StartTile :type "/Game/Blueprints/Board/Tile Structure") (DestinationTile :type "/Game/Blueprints/Board/Tile Structure"))
  (returns (Result :type Boolean))
  (locals (SelectedPiece :type "/Game/Blueprints/Pieces/BP_Piece Object Reference"))
  (bind _output_get (set `local.SelectedPiece` (`self.GetPieceAtTile` StartTile)))
  (`/Engine/EditorBlueprintResources/StandardMacros.IsValid` _output_get
    (:`Is Valid`
      (return (`KismetArrayLibrary.Array_Contains` (`/Game/Blueprints/Pieces/BP_Piece.GetAvailableMoves` (`local.SelectedPiece`) (`local.StartTile`)) (`local.DestinationTile`))))
    (:`Is Not Valid`
      (return false))))

(fn `Convert Tile to World`
  (params (Tile :type "/Game/Blueprints/Board/Tile Structure"))
  (returns (ReturnValue :type "Vector Structure"))
  (return (+ (`KismetMathLibrary.MakeVector` (+ (* Tile_Row_4_A31AD37F4ABEE7282C2022A30B0EBA3F (`self.TileWidth`)) (`self.HalfTileWidth`)) (+ (* Tile_Col_2_767D76F24B6395F8CD2202A2E588D57E (`self.TileWidth`)) (`self.HalfTileWidth`))) (`self.GetGridCorner`))))

(fn `ConvertWorldToGrid`
  (params (WorldLocation :type "Vector Structure"))
  (returns (Valid :type Boolean) (Tile :type "/Game/Blueprints/Board/Tile Structure"))
  (locals (`Row (local)` :type Integer :default 0) (`Col (local)` :type Integer :default 0))
  (bind _tilewidth (`self.TileWidth`))
  (bind (_returnvalue_x _returnvalue_y) (`KismetMathLibrary.BreakVector` (- (`local.WorldLocation`) (`self.GetGridCorner`))))
  (`|ExecutionSequence`
    (:`then_0`
      (set `local.Row (local)` (`KismetMathLibrary.FFloor` (/ _returnvalue_x _tilewidth)))
      (set `local.Col (local)` (`KismetMathLibrary.FFloor` (/ _returnvalue_y _tilewidth))))
    (:`then_1`
      (if (`self.IsValidTile?` (make `/Game/Blueprints/Board/Tile` (`local.Col (local)`) (`local.Row (local)`)))
        (return true (make `/Game/Blueprints/Board/Tile` (`local.Col (local)`) (`local.Row (local)`)))
        (else
          (return false))))))

(fn `GetGridCorner`
  (returns (ReturnValue :type "Vector Structure"))
  (bind (_returnvalue_x _returnvalue_y _returnvalue_z) (`KismetMathLibrary.BreakVector` (`self.K2_GetActorLocation`)))
  (return (`KismetMathLibrary.MakeVector` (- _returnvalue_x (* (`self.TileWidth`) 4.0)) (- _returnvalue_y (* (`self.TileWidth`) 4.0)) _returnvalue_z)))

(fn `GetPieceAtTile`
  (params (Tile :type "/Game/Blueprints/Board/Tile Structure"))
  (returns (Piece :type "/Game/Blueprints/Pieces/BP_Piece Object Reference"))
  (return (`|GetArrayItem` (`self.BoardState`) (`self.TileToIndex` Tile))))

(fn `GetRandomMove`
  (returns (StartingTile1 :type "/Game/Blueprints/Board/Tile Structure") (TargetTile1 :type "/Game/Blueprints/Board/Tile Structure"))
  (locals (StartingTile :type "/Game/Blueprints/Board/Tile Structure") (TargetTile :type "/Game/Blueprints/Board/Tile Structure") (Loop :type Boolean :default true) (Piece :type "/Game/Blueprints/Pieces/BP_Piece Object Reference"))
  (bind _startingtile (`local.StartingTile`))
  (bind _piece (`local.Piece`))
  (bind (_valid _tile) (`self.ConvertWorldToGrid` (`self.K2_GetActorLocation` _piece)))
  (bind _destinationtiles (`/Game/Blueprints/Pieces/BP_Piece.GetAvailableMoves` _piece _tile))
  (while (`local.Loop`)
    (bind _output_get (set `local.Piece` (`KismetArrayLibrary.Array_Random` (`self.BoardState`))))
    (`/Engine/EditorBlueprintResources/StandardMacros.IsValid` _output_get
      (:`Is Valid`
        (if (`KismetSystemLibrary.IsValid` _piece)
          (if (== 1 (`/Game/Blueprints/Pieces/BP_Piece.OwningPlayerIndex` _piece))
            (if _valid
              (set `local.StartingTile` _tile)
              (if (> (`KismetArrayLibrary.Array_Length` _destinationtiles) 0)
                (bind _output_get_2 (set `local.TargetTile` (`KismetArrayLibrary.Array_Random` _destinationtiles)))
                (bind _result (`self.CanPerformMove?` _startingtile _output_get_2))
                (if _result
                  (if (== (`/Game/Blueprints/Pieces/BP_Piece.OwningPlayerIndex` (`self.GetPieceAtTile` _startingtile)) 1)
                    (set `local.Loop` false))))))))))
  (return (`local.StartingTile`) (`local.TargetTile`)))

(fn `GetTileData`
  (params (Tile :type "/Game/Blueprints/Board/Tile Structure"))
  (returns (TileValid :type Boolean) (TileFree :type Boolean) (Piece :type "/Game/Blueprints/Pieces/BP_Piece Object Reference"))
  (bind _piece (`self.GetPieceAtTile` (`local.Tile`)))
  (if (`self.IsValidTile?` Tile)
    (return true (not (`KismetSystemLibrary.IsValid` _piece)) _piece)
    (else
      (return false false null))))

(fn `IsValidTile?`
  (params (Tile :type "/Game/Blueprints/Board/Tile Structure"))
  (returns (ReturnValue :type Boolean))
  (return (and (`KismetMathLibrary.InRange_IntInt` Tile_Col_2_767D76F24B6395F8CD2202A2E588D57E 0 7) (`KismetMathLibrary.InRange_IntInt` Tile_Row_4_A31AD37F4ABEE7282C2022A30B0EBA3F 0 7))))

(fn `PerformMove`
  (params (StartTile :type "/Game/Blueprints/Board/Tile Structure") (DestinationTile :type "/Game/Blueprints/Board/Tile Structure"))
  (locals (SelectedPiece :type "/Game/Blueprints/Pieces/BP_Piece Object Reference") (DestinationPiece :type "/Game/Blueprints/Pieces/BP_Piece Object Reference"))
  (set `local.SelectedPiece` (`self.GetPieceAtTile` StartTile))
  (set `local.DestinationPiece` (`self.GetPieceAtTile` DestinationTile))
  (`self.K2_SetActorLocation` (`local.SelectedPiece`) (`self.Convert Tile to World` (`local.DestinationTile`)) false true)
  (bind _destinationpiece (`local.DestinationPiece`)
    (:`then`
      (`self.K2_DestroyActor` _destinationpiece))
    (:`else`
      _))
  (`self.BoardStateMovePiece` (`local.StartTile`) (`local.DestinationTile`)))

(fn `Spawn Pawns`
  (params (PlayerIndex :type Integer))
  (locals (Row :type Integer) (Col :type Integer))
  (set `local.Row` (select `int` (`local.PlayerIndex`) :`0` 1 :`1` 6))
  (for _index (range 8)
    (bind _output_get (set `local.Col` _index))
    (bind _returnvalue (`|SpawnActorFromClass` "/Game/Blueprints/Pieces/BP_Pawn.BP_Pawn_C" (`KismetMathLibrary.MakeTransform` (`self.Convert Tile to World` (make `/Game/Blueprints/Board/Tile` _output_get (`local.Row`)))) "Undefined" "OverrideRootScale" null (`local.PlayerIndex`) null))
    (`self.BoardStateAddPiece` _returnvalue (make `/Game/Blueprints/Board/Tile` (`local.Col`) (`local.Row`)))))

(fn `SpawnBishops`
  (params (PlayerIndex :type Integer))
  (locals (Row :type Integer) (Col :type Integer))
  (set `local.Row` (select `int` (`local.PlayerIndex`) :`0` 0 :`1` 7))
  (`|ExecutionSequence`
    (:`then_0`
      ;[1 1 1] Left
      (set `local.Col` (select `int` (`local.PlayerIndex`) :`0` 2 :`1` 5))
      (bind _returnvalue (`|SpawnActorFromClass` "/Game/Blueprints/Pieces/BP_Bishop.BP_Bishop_C" (`KismetMathLibrary.MakeTransform` (`self.Convert Tile to World` (make `/Game/Blueprints/Board/Tile` (`local.Col`) (`local.Row`)))) "Undefined" "OverrideRootScale" null (`local.PlayerIndex`) null))
      (`self.BoardStateAddPiece` _returnvalue (make `/Game/Blueprints/Board/Tile` (`local.Col`) (`local.Row`))))
    (:`then_1`
      ;[1 1 1] Right
      (set `local.Col` (select `int` (`local.PlayerIndex`) :`0` 5 :`1` 2))
      (bind _returnvalue_2 (`|SpawnActorFromClass` "/Game/Blueprints/Pieces/BP_Bishop.BP_Bishop_C" (`KismetMathLibrary.MakeTransform` (`self.Convert Tile to World` (make `/Game/Blueprints/Board/Tile` (`local.Col`) (`local.Row`)))) "Undefined" "OverrideRootScale" null (`local.PlayerIndex`) null))
      (`self.BoardStateAddPiece` _returnvalue_2 (make `/Game/Blueprints/Board/Tile` (`local.Col`) (`local.Row`))))))

(fn `SpawnKings`
  (params (PlayerIndex :type Integer))
  (locals (Row :type Integer) (Col :type Integer))
  (set `local.Row` (select `int` (`local.PlayerIndex`) :`0` 0 :`1` 7))
  (set `local.Col` 4)
  (bind _returnvalue (`|SpawnActorFromClass` "/Game/Blueprints/Pieces/BP_King.BP_King_C" (`KismetMathLibrary.MakeTransform` (`self.Convert Tile to World` (make `/Game/Blueprints/Board/Tile` (`local.Col`) (`local.Row`)))) "Undefined" "OverrideRootScale" null (`local.PlayerIndex`) null))
  (`self.BoardStateAddPiece` _returnvalue (make `/Game/Blueprints/Board/Tile` (`local.Col`) (`local.Row`))))

(fn `SpawnKnights`
  (params (PlayerIndex :type Integer))
  (locals (Row :type Integer) (Col :type Integer))
  (set `local.Row` (select `int` (`local.PlayerIndex`) :`0` 0 :`1` 7))
  (`|ExecutionSequence`
    (:`then_0`
      ;[1 1 1] Left
      (set `local.Col` (select `int` (`local.PlayerIndex`) :`0` 1 :`1` 6))
      (bind _returnvalue (`|SpawnActorFromClass` "/Game/Blueprints/Pieces/BP_Knight.BP_Knight_C" (`KismetMathLibrary.MakeTransform` (`self.Convert Tile to World` (make `/Game/Blueprints/Board/Tile` (`local.Col`) (`local.Row`)))) "Undefined" "OverrideRootScale" null (`local.PlayerIndex`) null))
      (`self.BoardStateAddPiece` _returnvalue (make `/Game/Blueprints/Board/Tile` (`local.Col`) (`local.Row`))))
    (:`then_1`
      ;[1 1 1] Right
      (set `local.Col` (select `int` (`local.PlayerIndex`) :`0` 6 :`1` 1))
      (bind _returnvalue_2 (`|SpawnActorFromClass` "/Game/Blueprints/Pieces/BP_Knight.BP_Knight_C" (`KismetMathLibrary.MakeTransform` (`self.Convert Tile to World` (make `/Game/Blueprints/Board/Tile` (`local.Col`) (`local.Row`)))) "Undefined" "OverrideRootScale" null (`local.PlayerIndex`) null))
      (`self.BoardStateAddPiece` _returnvalue_2 (make `/Game/Blueprints/Board/Tile` (`local.Col`) (`local.Row`))))))

(fn `SpawnQueens`
  (params (PlayerIndex :type Integer))
  (locals (Row :type Integer) (Col :type Integer))
  (set `local.Row` (select `int` (`local.PlayerIndex`) :`0` 0 :`1` 7))
  (set `local.Col` 3)
  (bind _returnvalue (`|SpawnActorFromClass` "/Game/Blueprints/Pieces/BP_Queen.BP_Queen_C" (`KismetMathLibrary.MakeTransform` (`self.Convert Tile to World` (make `/Game/Blueprints/Board/Tile` (`local.Col`) (`local.Row`)))) "Undefined" "OverrideRootScale" null (`local.PlayerIndex`) null))
  (`self.BoardStateAddPiece` _returnvalue (make `/Game/Blueprints/Board/Tile` (`local.Col`) (`local.Row`))))

(fn `SpawnRooks`
  (params (PlayerIndex :type Integer))
  (locals (Row :type Integer) (Col :type Integer))
  (set `local.Row` (select `int` (`local.PlayerIndex`) :`0` 0 :`1` 7))
  (`|ExecutionSequence`
    (:`then_0`
      ;[1 1 1] Left
      (set `local.Col` (select `int` (`local.PlayerIndex`) :`0` 0 :`1` 7))
      (bind _returnvalue (`|SpawnActorFromClass` "/Game/Blueprints/Pieces/BP_Rook.BP_Rook_C" (`KismetMathLibrary.MakeTransform` (`self.Convert Tile to World` (make `/Game/Blueprints/Board/Tile` (`local.Col`) (`local.Row`)))) "Undefined" "OverrideRootScale" null (`local.PlayerIndex`) null))
      (`self.BoardStateAddPiece` _returnvalue (make `/Game/Blueprints/Board/Tile` (`local.Col`) (`local.Row`))))
    (:`then_1`
      ;[1 1 1] Right
      (set `local.Col` (select `int` (`local.PlayerIndex`) :`0` 7 :`1` 0))
      (bind _returnvalue_2 (`|SpawnActorFromClass` "/Game/Blueprints/Pieces/BP_Rook.BP_Rook_C" (`KismetMathLibrary.MakeTransform` (`self.Convert Tile to World` (make `/Game/Blueprints/Board/Tile` (`local.Col`) (`local.Row`)))) "Undefined" "OverrideRootScale" null (`local.PlayerIndex`) null))
      (`self.BoardStateAddPiece` _returnvalue_2 (make `/Game/Blueprints/Board/Tile` (`local.Col`) (`local.Row`))))))

(fn `UserConstructionScript`)