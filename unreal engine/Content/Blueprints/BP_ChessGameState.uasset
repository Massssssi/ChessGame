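; Game state for a networked chess game that tracks turns across three boards: Bot 1, Bot 2 and PvP.
; On BeginPlay it caches each BP_Board by type for board lookup and mouse-trace tile picking.
; A server event toggles the given board's active player, then multicasts the turn start to fire OnActivePlayerSet.
; The multicast always writes the PvP index, whatever the board, and the delayed first-turn start is unwired.
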(event `self.ReceiveBeginPlay`
  (bind _outactors (`GameplayStatics.GetAllActorsOfClass` "/Game/Blueprints/Board/BP_Board.BP_Board_C"))
  (for _array_element _outactors
    (switch `/Game/Blueprints/Board/E_BoardType` (`/Game/Blueprints/Board/BP_Board.Type` _array_element)
      (:`NewEnumerator0`
        (set `self.Bot1Board` _array_element))
      (:`NewEnumerator1`
        (set `self.Bot2Board` _array_element))
      (:`NewEnumerator2`
        (set `self.PvPBoard` _array_element)))))

(event `BeginPlayerTurn (multi)`
  (params (PlayerIndex :type Integer) (Board :type "/Game/Blueprints/Board/E_BoardType Enum" :default "NewEnumerator0"))
  (bind _output_get (set `self.ActivePlayerIndexPvP` PlayerIndex))
  (`self.OnActivePlayerSet` _output_get Board))

(event `EndPlayerTurn (server)`
  (params (Board :type "/Game/Blueprints/Board/E_BoardType Enum" :default "NewEnumerator0"))
  (switch `/Game/Blueprints/Board/E_BoardType` Board
    (:`NewEnumerator0`
      (if (== (`self.ActivePlayerIndexBot1`) 0)
        (set `self.ActivePlayerIndexBot1` 1)
        (else
          (set `self.ActivePlayerIndexBot1` 0)))
      (`self.BeginPlayerTurn (multi)` (`self.ActivePlayerIndexBot1`)))
    (:`NewEnumerator1`
      (if (== (`self.ActivePlayerIndexBot2`) 0)
        (set `self.ActivePlayerIndexBot2` 1)
        (else
          (set `self.ActivePlayerIndexBot2` 0)))
      (`self.BeginPlayerTurn (multi)` (`self.ActivePlayerIndexBot2`) "NewEnumerator1"))
    (:`NewEnumerator2`
      (if (== (`self.ActivePlayerIndexPvP`) 0)
        (set `self.ActivePlayerIndexPvP` 1)
        (else
          (set `self.ActivePlayerIndexPvP` 0)))
      (`self.BeginPlayerTurn (multi)` (`self.ActivePlayerIndexPvP`) "NewEnumerator2"))))

(fn `GetActivePlayerIndex`
  (returns (ActivePlayerIndex :type Integer))
  (return (`self.ActivePlayerIndexPvP`)))

(fn `GetBoard`
  (params (BoardType :type "/Game/Blueprints/Board/E_BoardType Enum" :default "NewEnumerator0"))
  (returns (Board :type "/Game/Blueprints/Board/BP_Board Object Reference"))
  (return (select `/Game/Blueprints/Board/E_BoardType` BoardType :`NewEnumerator0` (`self.Bot1Board`) :`NewEnumerator1` (`self.Bot2Board`) :`NewEnumerator2` (`self.PvPBoard`))))

(fn `GetHoveredTile`
  (params (PlayerController :type "PlayerController Object Reference") (Board :type "/Game/Blueprints/Board/E_BoardType Enum" :default "NewEnumerator0"))
  (returns (Valid :type Boolean) (Tile :type "/Game/Blueprints/Board/Tile Structure"))
  (bind (_worldlocation _worlddirection) (`PlayerController.DeprojectMousePositionToWorld` PlayerController))
  (bind (_outhit _returnvalue) (`KismetSystemLibrary.LineTraceSingle` _worldlocation (+ _worldlocation (* _worlddirection 10000.0)) "TraceTypeQuery1"))
  (if _returnvalue
    (bind (_valid _tile) (`/Game/Blueprints/Board/BP_Board.ConvertWorldToGrid` (select `/Game/Blueprints/Board/E_BoardType` Board :`NewEnumerator0` (`self.Bot1Board`) :`NewEnumerator1` (`self.Bot2Board`) :`NewEnumerator2` (`self.PvPBoard`)) (`.Location` (`GameplayStatics.BreakHitResult` _outhit))))
    (return _valid _tile)
    (else
      (return false))))

(fn `UserConstructionScript`)