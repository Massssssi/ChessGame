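; Chess game mode that sets up matches for two connected players, either against each other or each against AI.
; Once the second player logs in, a looping timer polls both controllers' chosen modes.
; If both pick PvP, it pauses the timer, assigns indices, clears widgets and starts a shared board through the game state.
; Otherwise, each player choosing AI starts once on a separate board as player index 0.
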(event `self.K2_PostLogin`
  (params (NewPlayer :type "PlayerController Object Reference"))
  (`parent.K2_PostLogin` NewPlayer)
  (bind _returnvalue (`self.GetNumPlayers`))
  (if (== _returnvalue 2)
    (bind _returnvalue_2 (`KismetSystemLibrary.K2_SetTimerDelegate` (delegate `WaitForPlayers`) 0.2 true))
    (set `self.Handle` _returnvalue_2)))

(event `WaitForPlayers`
  (bind _playercontroller (`self.GetPlayer` 0))
  (bind _playercontroller_2 (`self.GetPlayer` 1))
  (bind _playercontroller_3 (`self.GetPlayer` 0))
  (bind _asbp_chess_game_state (cast `/Game/Blueprints/BP_ChessGameState` (`GameplayStatics.GetGameState`) :!pure true))
  (if (and (`KismetSystemLibrary.IsValid` _playercontroller_3) (`KismetSystemLibrary.IsValid` _playercontroller_2))
    (if (and (`/Game/Blueprints/BP_PlayerController.Play Against Player` _playercontroller_3) (`/Game/Blueprints/BP_PlayerController.Play Against Player` _playercontroller_2))
      (`KismetSystemLibrary.K2_PauseTimerHandle` (`self.Handle`))
      (`KismetSystemLibrary.Delay` 0.5)
      (`|ExecutionSequence`
        (:`then_0`
          (`self.Assign Player Indices`))
        (:`then_1`
          (`/Game/Blueprints/BP_PlayerController.RemoveWidget` _playercontroller)
          (`/Game/Blueprints/BP_PlayerController.RemoveWidget` (`self.GetPlayer` 1))
          (`/Game/Blueprints/BP_PlayerController.SetBoard` _playercontroller "NewEnumerator2")
          (`/Game/Blueprints/BP_PlayerController.SetBoard` (`self.GetPlayer` 1) "NewEnumerator2")
          (`/Game/Blueprints/BP_ChessGameState.BeginPlayerTurn (multi)` _asbp_chess_game_state 0 "NewEnumerator2")))
      (elif (`/Game/Blueprints/BP_PlayerController.PlayAgainstAI` _playercontroller_3)
        (`|ExecutionSequence`
          (:`then_0`
            (`/Engine/EditorBlueprintResources/StandardMacros.DoOnce` false
              (:`Completed`
                (`/Game/Blueprints/BP_PlayerController.SetPlayerIndex (client)` _playercontroller_3 0)
                (`/Game/Blueprints/BP_PlayerController.SetBoard` _playercontroller "NewEnumerator0")
                (`/Game/Blueprints/BP_ChessGameState.BeginPlayerTurn (multi)` _asbp_chess_game_state 0 "NewEnumerator0"))))
          (:`then_1`
            (if (`/Game/Blueprints/BP_PlayerController.PlayAgainstAI` _playercontroller_2) :!label _label
              (`/Engine/EditorBlueprintResources/StandardMacros.DoOnce` false
                (:`Completed`
                  (`/Game/Blueprints/BP_PlayerController.SetPlayerIndex (client)` _playercontroller_2 0)
                  (`/Game/Blueprints/BP_PlayerController.SetBoard` (`self.GetPlayer` 1) "NewEnumerator1")
                  (`/Game/Blueprints/BP_ChessGameState.BeginPlayerTurn (multi)` _asbp_chess_game_state 0 "NewEnumerator1"))))))
        (else
          (goto _label))))))

(fn `Assign Player Indices`
  (`/Game/Blueprints/BP_PlayerController.SetPlayerIndex (client)` (`self.GetPlayer` 0) 0)
  (`/Game/Blueprints/BP_PlayerController.SetPlayerIndex (client)` (`self.GetPlayer` 1) 1))

(fn `UserConstructionScript`)