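; Chess function library that provides shared helpers for player colors and access to chess game objects.
; Player index 0 maps to near-white and 1 to near-black, and the opponent lookup swaps the index before reusing that mapping.
; Board lookup casts the current game state to BP_ChessGameState and asks it for the board of the requested type.
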(fn `GetBoard`
  (params (BoardType :type "/Game/Blueprints/Board/E_BoardType Enum" :default "NewEnumerator0"))
  (returns (Board :type "/Game/Blueprints/Board/BP_Board Object Reference"))
  (return (`/Game/Blueprints/BP_ChessGameState.GetBoard` (`self.GetChessGameState` (`local.__WorldContext`)) BoardType)))

(fn `GetChessGameState`
  (returns (`Chess Game State` :type "/Game/Blueprints/BP_ChessGameState Object Reference"))
  (return (cast `/Game/Blueprints/BP_ChessGameState` (`GameplayStatics.GetGameState` null) :!pure true)))

(fn `GetOpponentColor`
  (params (PlayerIndex :type Integer))
  (returns (NewParam :type "LinearColor Structure"))
  (return (`self.GetPlayerColor` (select `int` PlayerIndex :`0` 1 :`1` 0) (`local.__WorldContext`))))

(fn `GetPlayerColor`
  (params (PlayerIndex :type Integer))
  (returns (NewParam :type "LinearColor Structure"))
  (return (select `int` PlayerIndex :`0` (struct :`R` 0.9 :`G` 0.9 :`B` 0.9 :`A` 1.0) :`1` (struct :`R` 0.01 :`G` 0.01 :`B` 0.01 :`A` 1.0) :!type "LinearColor Structure")))